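; BP_Buton is an interactable button that opens and closes a linked plate (BPPLAKA) and animates its own movement.
; Each OnInteract alternates between OpenPlate and ClosePlate through a FlipFlop.
; A separate boolean, InAnimationCompleted, toggles the Buton_Hareketi timeline between Play and Reverse, which drives the Cube's relative Z location.
; The boolean flips when playback starts, without waiting for the timeline to finish.
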(event OnComponentBeginOverlap(Cube)
  (params (OverlappedComponent :type Primitive%20Component%20Object%20Reference) (OtherActor :type Actor%20Object%20Reference) (OtherComp :type Primitive%20Component%20Object%20Reference) (OtherBodyIndex :type Integer) (bFromSweep :type Boolean) (SweepResult :type Hit%20Result%20Structure%20%28by%20ref%29)))

(event EventBeginPlay)

(event EventOnInteract
  (Utilities|FlowControl|FlipFlop
    (:A
      (Default|OpenPlate (Variables|Default|GetBP_PLAKA)))
    (:B
      (Default|ClosePlate (Variables|Default|GetBP_PLAKA))))
  (if (Variables|Default|GetInAnimationCompleted)
    (Variables|Default|SetInAnimationCompleted false)
    (bind _newtrack_0 (Timeline|Buton_Hareketi Reverse)
      (:Update
        (Transformation|SetRelativeLocation (Variables|Default|GetCube) (Math|Vector|MakeVector 0.0 0.0 _newtrack_0) false false)))
    (else
      (Variables|Default|SetInAnimationCompleted true)
      (Timeline|Buton_Hareketi Play))))

(fn ConstructionScript)